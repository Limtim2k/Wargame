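; Base weapon for units and buildings that fires shot actors on a looping timer and draws ammo from its owner.
; BeginPlay casts the owner to a main building, falling back to a main unit, to pick which ammo pool to use.
; Start and end events set or clear the rate-of-fire timer.
; Each shot checks overheating, a random reliability roll and ammo, then spawns BP_base_shot and adds heat, with no cooldown here.
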(event `self.ReceiveBeginPlay`
  (bind _returnvalue (`self.GetOwner`))
  ;[1 1 1] Инициализация
  (bind _asbp_main_building (cast `/Game/main/Buildings/main/BP_main_building` _returnvalue)
    (:`then`
      (set `self.Building` _asbp_main_building))
    (:`CastFailed`
      (set `self.Unit` (cast `/Game/main/Units/main_Unit/BP_main_unit` _returnvalue :!pure true))
      (set `self.Unit?` true))))

(event `End weapon`
  (`KismetSystemLibrary.K2_ClearAndInvalidateTimerHandle` (stale `Start weapon` _returnvalue)))

(event `Start weapon`
  (bind _returnvalue (`KismetSystemLibrary.K2_SetTimerDelegate` (delegate `Fire`) (`.Rateoffire_2_A05AB81E48A9B6191E015E86DE9B8AA3` (break `/Game/main/Units/ST_base_weapon` (`self.Weapon`))) true)))

(event `Fire`
  (bind ((`Overheating_4_FAF6E7684F8DD8001A125BAD4E16DAF7` _overheating) (`OverHeatingMax_14_1BF070E446420D299659D895779663FA` _overheatingmax)) (break `/Game/main/Units/ST_base_weapon` (`self.Weapon`)))
  (if (>= _overheating _overheatingmax)
    (`KismetSystemLibrary.PrintString` "Перегрев")
    (else
      ;[1 1 1] Надеженость
      (bind _returnvalue (`self.Reliability`))
      (if _returnvalue
        (`KismetSystemLibrary.PrintString` "FAIL. use")
        (else
          ;[1 1 1] Использование патронов
          (bind _useammo_ (`self.Use ammo`))
          (if _useammo_
            ;[1 1 1] Создание пуль
            (`|SpawnActorFromClass` "/Game/main/Units/BP_base_shot.BP_base_shot_C" (`self.Spawn location`) "Undefined" "OverrideRootScale" null 0.0 null)
            (`/Engine/EditorBlueprintResources/StandardMacros.IncrementFloat` (`.Overheating_4_FAF6E7684F8DD8001A125BAD4E16DAF7` (break `/Game/main/Units/ST_base_weapon` (`self.Weapon`))))))))))

(fn `Reliability`
  (returns (ReturnValue :type Boolean))
  (return (> (`KismetMathLibrary.RandomFloatInRange` 0.0 100.0) (`.Reliability_11_00CCD81F4E980A9F3D3432857F3F8AC5` (break `/Game/main/Units/ST_base_weapon` (`self.Weapon`))))))

(fn `Use ammo`
  (returns (`UseAmmo?` :type Boolean))
  (bind _spetifications (`/Game/main/Units/main_Unit/BP_main_unit.Spetifications` (`self.Unit`)))
  (bind _building (`/Game/main/Buildings/main/BP_main_building.Building` (`self.Building`)))
  (bind ((`Ammo_15_C271830F488EAE2D264587A1C0779184` _ammo)) (break `/Game/main/Units/main_Unit/ST_main_unit_spetifications` _spetifications))
  (bind ((`Building_visual_29_F483B7A54908CE050FFB50A508EB6D17` _building_visual) (`Ammo_20_144082024BD2E4042D5D95B8031D303A` _ammo_2)) (break `/Game/main/Buildings/main/ST_main_building` _building))
  (if (`self.Unit?`)
    (if (> _ammo 0)
      (bind _result (`/Engine/EditorBlueprintResources/StandardMacros.DecrementInt` _ammo)
        (:`  `
          (setmembers `/Game/main/Units/main_Unit/ST_main_unit_spetifications` :`StructRef` _spetifications :`Ammo` _result)
          (return true)))
      (else
        _))
    (elif (> _ammo_2 0)
      (bind _result_2 (`/Engine/EditorBlueprintResources/StandardMacros.DecrementInt` _ammo_2)
        (:`  `
          (setmembers `/Game/main/Buildings/main/ST_main_building` :`StructRef` _building :`Ammo` _result_2)
          (return true)))
      (else
        _)))
  (`KismetSystemLibrary.PrintString` "NO ammo")
  (return false))

(fn `UserConstructionScript`)
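; BP_main_unit is a unit actor with HP and armor that is destroyed when its HP runs out.
; Incoming damage goes to DamageSystem, where the BP_base_type_damage object computes the applied amount.
; Results of -0.1 or lower are added directly to HP in the Spetifications struct; others are subtracted after armor reduction.
; Tick with a Delay also makes the unit periodically apply ammo-type damage to itself.
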(event `self.ReceiveTick`
  (params (DeltaSeconds :type "Float (single-precision)"))
  (`KismetSystemLibrary.Delay` 0.6)
  (`GameplayStatics.ApplyDamage` self 2.0 null null "/Game/main/Other/Damage/BP_type_damage_ammo.BP_type_damage_ammo_C"))

(event `self.ReceiveAnyDamage`
  (params (Damage :type "Float (single-precision)") (DamageType :type "DamageType Object Reference") (InstigatedBy :type "Controller Object Reference") (DamageCauser :type "Actor Object Reference"))
  ;[1 1 1] Смерть и урон
  (`self.Damage system` Damage DamageType))

(fn `Damage system`
  (params (Damage :type "Float (double-precision)") (DamageType :type "DamageType Object Reference"))
  (locals (HP :type "Float (double-precision)") (Armor :type "Float (double-precision)"))
  (bind (_hp _maxhp _armor) (break `/Game/main/Units/main_Unit/ST_main_unit_spetifications` (`self.Spetifications`)))
  (set `local.HP` _hp)
  (set `local.Armor` _armor)
  (bind _damageout (`/Game/main/Other/Damage/BP_base_type_damage.Apply damage` (cast `/Game/main/Other/Damage/BP_base_type_damage` DamageType :!pure true) Damage))
  (if (<= _damageout -0.1)
    (setmembers `/Game/main/Units/main_Unit/ST_main_unit_spetifications` :`StructRef` (`self.Spetifications`) :`HP` (+ (`local.HP`) _damageout))
    (else
      (setmembers `/Game/main/Units/main_Unit/ST_main_unit_spetifications` :`StructRef` (`self.Spetifications`) :`HP` (- (`local.HP`) (- _damageout (`local.Armor`))))))
  (if (<= (`local.HP`) 0.0)
    (`self.K2_DestroyActor`)))

(fn `UserConstructionScript`)
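; RTS-style player controller that drives the BP_player camera pawn and starts or ends unit selection with the left mouse button.
; Mouse wheel plays timelines that offset the pawn vertically.
; The engeControll graph turns cursor proximity to viewport edges into scroll speed, applied as XY offset from the Mouse X event.
; Line-trace click selection, filtered by CommandIndex into UnitsSelect, exists but is disconnected.
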(event `InputAxisKey|MouseWheelAxis`
  (params (AxisValue :type "Float (single-precision)"))
  ;[1 1 1] ВВерх вниз
  (if (== AxisValue 1.0)
    (bind (_direction _newtrack_0) (`Timeline|Timeline_1` :!via `PlayFromStart`)
      (:`Update`
        (`self.K2_AddActorWorldOffset` (`self.Player pawn`) (`KismetMathLibrary.MakeVector` 0.0 0.0 _newtrack_0) false false)))
    (elif (== AxisValue -1.0)
      (bind (_direction_2 _newtrack_0_2) (`Timeline|Timeline_0` :!via `PlayFromStart`)
        (:`Update`
          (`self.K2_AddActorWorldOffset` (`self.Player pawn`) (`KismetMathLibrary.MakeVector` 0.0 0.0 _newtrack_0_2) false false))))))

(event `self.ReceiveBeginPlay`
  ;[1 1 1] Инициализация
  (set `self.Player pawn` (cast `/Game/main/Player/BP_player` (`GameplayStatics.GetPlayerPawn` 0) :!pure true)))

(event `InputAxis|Mouse X`
  (params (AxisValue :type "Float (single-precision)"))
  (bind (_y _x) (`self.Enge controll` :!label _label)
    (:`NewParam`
      (`self.K2_AddActorWorldOffset` (`self.Player pawn`) (`KismetMathLibrary.MakeVector` _x _y) false false))))

(event `InputAxis|Mouse Y`
  (params (AxisValue :type "Float (single-precision)"))
  (goto _label :!via `Mouse Y`))

(event `Key|LeftMouseButton`
  (params (Key :type "Key Structure"))
  (:`Pressed`
    (`self.Start selection`))
  (:`Released`
    (`self.End selection`)))

(fn `Add units to select`
  (params (Unit :type "/Game/main/Units/BP_main_unit Object Reference"))
  (`KismetArrayLibrary.Array_Add` (`self.Units select`) Unit))

(fn `Click units`
  (returns (Actor :type "Actor Object Reference"))
  (bind (_locationx _locationy) (`self.GetMousePosition`))
  (bind _returnvalue (`SceneComponent.K2_GetComponentLocation` (`/Game/main/Player/BP_player.Camera` (`self.Player pawn`))))
  (bind _outhit (`KismetSystemLibrary.LineTraceSingle` _returnvalue (+ _returnvalue (* (`.WorldDirection` (`GameplayStatics.DeprojectScreenToWorld` self (`KismetMathLibrary.MakeVector2D` _locationx _locationy))) (1000000.0 1000000.0 1000000.0))) "TraceTypeQuery3"))
  (return (`.HitActor` (`GameplayStatics.BreakHitResult` _outhit))))

(fn `Find unit`
  (params (Unit :type "/Game/main/Units/BP_main_unit Object Reference"))
  (returns (`Find?` :type Boolean))
  (return (== (`KismetArrayLibrary.Array_Find` (`self.Units select`) Unit) 0)))

(fn `manangment unit`
  (params (Object :type "Object Object Reference"))
  (locals (Unit :type "/Game/main/Units/BP_main_unit Object Reference"))
  (bind _asbp_main_unit (cast `/Game/main/Units/BP_main_unit` Object))
  (if (== (`/Game/main/Units/BP_main_unit.Command Index` _asbp_main_unit) (`self.Command Index`))
    (bind _output_get (set `local.Unit` _asbp_main_unit))
    (if (`self.Find unit` _output_get)
      (`KismetSystemLibrary.PrintString` "Find")
      (else
        (`self.Add units to select` (`local.Unit`))
        (`KismetSystemLibrary.PrintString` "666")))))

(fn `UserConstructionScript`)
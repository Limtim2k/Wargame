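; BP_energy_net is an actor representing one energy network, holding the grid members that belong to it and starting with its owner.
; A Newnet event merges it with another net through ConnectNet, which compares member counts and picks randomly on a tie.
; AddNet appends one member array to the other, repoints each member's EnergyNet to the surviving net and destroys the absorbed net actor.
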(event `New net`
  (params (`New net` :type "/Game/main/Buildings/Energy_grid/BP_energy_net Object Reference"))
  ;[1 1 1] Объединение сетей
  (`/Engine/EditorBlueprintResources/StandardMacros.IsValid` `New net`
    (:`Is Valid`
      (`self.Connect net` (`/Game/main/Buildings/Energy_grid/BP_energy_net.Energy greeds` `New net`) `New net`))))

(event `self.ReceiveBeginPlay`
  (`KismetArrayLibrary.Array_Add` (`self.Energy greeds`) (cast `/Game/main/Buildings/Energy_grid/BP_base_energy_grid` (`self.GetOwner`) :!pure true))
  (`KismetSystemLibrary.PrintString` "сеть создана"))

(event `self.ReceiveTick`
  (params (DeltaSeconds :type "Float (single-precision)"))
  (`KismetSystemLibrary.Delay` 5.0))

(fn `Add net`
  (params (`A+B?` :type Boolean) (A :type "Array of /Game/main/Buildings/Energy_grid/BP_base_energy_grid Object Reference (by ref)") (B :type "Array of /Game/main/Buildings/Energy_grid/BP_base_energy_grid Object Reference (by ref)") (`New net` :type "/Game/main/Buildings/Energy_grid/BP_energy_net Object Reference (by ref)"))
  (if `A+B?`
    ;[1 1 1] Старая сеть
    (`KismetArrayLibrary.Array_Append` A B)
    (for (_array_element _array_index) A
      (set `/Game/main/Buildings/Energy_grid/BP_base_energy_grid.Energy net` self (cast `/Game/main/Buildings/Energy_grid/BP_base_energy_grid` _array_element :!pure true)))
    (`self.K2_DestroyActor` `New net`)
    (`KismetSystemLibrary.PrintString` (`KismetStringLibrary.Conv_IntToString` _array_index))
    (else
      ;[1 1 1] Новая сеть
      (`KismetArrayLibrary.Array_Append` B A)
      (for (_array_element_2 _array_index_2) B
        (set `/Game/main/Buildings/Energy_grid/BP_base_energy_grid.Energy net` `New net` (cast `/Game/main/Buildings/Energy_grid/BP_base_energy_grid` _array_element_2 :!pure true))
        (`self.K2_DestroyActor`))
      (`self.K2_DestroyActor`)
      (`KismetSystemLibrary.PrintString` (`KismetStringLibrary.Conv_IntToString` _array_index_2)))))

(fn `Connect net`
  (params (`Energy greeds` :type "Array of /Game/main/Buildings/Energy_grid/BP_base_energy_grid Object Reference (by ref)") (Newnet :type "/Game/main/Buildings/Energy_grid/BP_energy_net Object Reference (by ref)"))
  (locals (`Energy greeds new` :type "Array of /Game/main/Buildings/Energy_grid/BP_base_energy_grid Object Reference") (`Energy net` :type "/Game/main/Buildings/Energy_grid/BP_energy_net Object Reference"))
  (bind _returnvalue (`KismetArrayLibrary.Array_Length` (`local.Energy greeds new`)))
  (bind _returnvalue_2 (`KismetArrayLibrary.Array_Length` (`self.Energy greeds`)))
  (set `local.Energy net` Newnet)
  (bind _output_get (set `local.Energy greeds new` `Energy greeds`))
  (if (== (`KismetArrayLibrary.Array_Length` (`self.Energy greeds`)) (`KismetArrayLibrary.Array_Length` _output_get))
    ;[1 1 1] Случайный выбор сети
    (`self.Add net` (`KismetMathLibrary.RandomBool`) (`self.Energy greeds`) (`local.Energy greeds new`) (`local.Energy net`))
    (`KismetSystemLibrary.PrintString` "случайный выбор")
    (else
      (`KismetSystemLibrary.PrintString` (`KismetStringLibrary.Concat_StrStr` (`KismetStringLibrary.Conv_IntToString` _returnvalue_2) (`KismetStringLibrary.Conv_IntToString` _returnvalue)))
      (if (>= _returnvalue_2 _returnvalue)
        (`self.Add net` true (`self.Energy greeds`) (`local.Energy greeds new`) (`local.Energy net`))
        (`KismetSystemLibrary.PrintString` "старая сеть больше")
        (else
          (`self.Add net` false (`self.Energy greeds`) (`local.Energy greeds new`) (`local.Energy net`))
          (`KismetSystemLibrary.PrintString` "старая сеть меньше"))))))

(fn `UserConstructionScript`)
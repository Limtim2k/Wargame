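; BP_base_energy_grid is a base building actor that forms part of an energy grid by linking with overlapping grid actors.
; On BeginPlay it spawns its own BP_energy_net and starts a looping five-second timer.
; Each tick of that timer scans its Box for other grid actors and, where nets differ, calls NewNet on the neighbor's net, passing its own.
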(event `self.ReceiveBeginPlay`
  (`parent.ReceiveBeginPlay`)
  (`KismetSystemLibrary.K2_SetTimerDelegate` (delegate `Find new energy grid`) 5.0 true)
  ;[1 1 1] Создание новой сети
  (bind _returnvalue (`|SpawnActorFromClass` "/Game/main/Buildings/Energy_grid/BP_energy_net.BP_energy_net_C" (`KismetMathLibrary.MakeTransform` (0.0 0.0 0.0)) "Undefined" "OverrideRootScale" self null))
  (set `self.Energy net` _returnvalue))

(event `Find new energy grid`
  (bind _energy_net (`self.Energy net`))
  (bind _overlappingactors (`PrimitiveComponent.GetOverlappingActors` (`self.Box`) "BP_base_energy_grid_C"))
  (if (`KismetArrayLibrary.Array_IsValidIndex` _overlappingactors)
    (for _array_element _overlappingactors
      (bind _asbp_base_energy_grid (cast `/Game/main/Buildings/Energy_grid/BP_base_energy_grid` _array_element :!pure true))
      (if (not (== _asbp_base_energy_grid self))
        (bind _energy_net_2 (`/Game/main/Buildings/Energy_grid/BP_base_energy_grid.Energy net` _asbp_base_energy_grid))
        (if (not (== _energy_net _energy_net_2))
          (`/Game/main/Buildings/Energy_grid/BP_energy_net.New net` _energy_net_2 _energy_net))))))

(fn `UserConstructionScript`
  (`parent.UserConstructionScript`))
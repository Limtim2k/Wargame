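; BP_main_building is a base building that produces and consumes resources for its owning player.
; A looping one-second timer adds generator fuel, material and ammo to the player state, subtracts fuel consumption, then refreshes the controller's UI.
; Material consumption is wired in reverse, decrementing the building's consumer value by player material.
; Capture switches owner references; the power-grid check and overlap search exist but are unconnected.
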(event `Capture`
  (params (NewParam :type "/Game/main/Player/BP_player Object Reference"))
  ;[1 1 1] Захват
  (bind _output_get (set `self.owner player` NewParam))
  (set `self.Player state` (cast `/Game/main/Player/BP_player_state` (`Pawn.PlayerState` _output_get) :!pure true))
  (set `self.Controller` (cast `/Game/main/Player/BP_controller` (`Pawn.GetController` (`self.owner player`)) :!pure true)))

(event `self.ReceiveBeginPlay`
  ;[1 1 1] Инициализация
  (set `self.Player state` (cast `/Game/main/Player/BP_player_state` (`Pawn.PlayerState` (`self.owner player`)) :!pure true))
  (set `self.Controller` (cast `/Game/main/Player/BP_controller` (`Pawn.GetController` (`self.owner player`)) :!pure true))
  (`KismetSystemLibrary.K2_SetTimerDelegate` (delegate `New cycle`) 1.0 true))

(event `New cycle`
  ;[1 1 1] Цикл
  ;;[1 1 1] Производство/потребление
  (`self.Resoursec `)
  (`self.UI_update`))

(fn `calculate`
  (params (Variable :type "Integer (by ref)") (`How many` :type Integer) (`Positive?` :type Boolean))
  (if `Positive?`
    (`|VariableSetRef` Variable (+ Variable `How many`))
    (else
      (`|VariableSetRef` Variable (- Variable `How many`)))))

(fn `Find power grid`
  (bind _overlappingactors (`PrimitiveComponent.GetOverlappingActors` (`self.Box`) "/Game/main/Buildings/Energy_grid/BP_base_energy_grid.BP_base_energy_grid_C"))
  (if (`KismetArrayLibrary.Array_IsValidIndex` _overlappingactors)
    (set `self.Power grid` (cast `/Game/main/Buildings/Energy_grid/BP_base_energy_grid` (`|GetArrayItem` _overlappingactors) :!pure true))
    (else
      (`KismetSystemLibrary.PrintString` "not find power grid"))))

(fn `Resoursec `
  (bind _player_state (`self.Player state`))
  (bind _player_state_2 (`self.Player state`))
  (bind ((`Generator_14_9F01D45F4CB547707543C4BFE2ED73F1` _generator) (`Consumer_17_C501CA344F7B46577A58F1AF13841A5D` _consumer)) (break `/Game/main/Buildings/main/ST_main_building` (`self.Building`)))
  (bind (_fuelgen _materialgen _energygen _ammo) (break `/Game/main/Buildings/main/ST_resources_building_generator` _generator))
  (bind (_materialconsumer _fuelconsumer) (break `/Game/main/Buildings/main/ST_consumption_building` _consumer))
  (`self.calculate` (`/Game/main/Player/BP_player_state.Fuel` _player_state) _fuelgen true)
  (`self.calculate` (`/Game/main/Player/BP_player_state.Material` _player_state) _materialgen true)
  (`self.calculate` (`/Game/main/Player/BP_player_state.Ammo` _player_state) _ammo true)
  (`self.calculate` _materialconsumer (`/Game/main/Player/BP_player_state.Material` _player_state_2))
  (`self.calculate` (`/Game/main/Player/BP_player_state.Fuel` _player_state_2) _fuelconsumer))

(fn `UI_update`
  (`/Game/main/UI/UI_player.UI_player_update_res` (`/Game/main/Player/BP_controller.UI` (`self.Controller`))))

(fn `UserConstructionScript`)